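; BP_Zombie is an enemy that roams randomly and chases any pawn it sees.
; Patrol loops AI moves to random reachable points, while PawnSensing triggers a chase ending in a neck-bite montage.
; The montage notify runs a forward sphere trace to damage the target's HealthComponent, with CanAttack gating repeats.
; Health's death event disables collision and movement, plays a death montage and destroys the actor; the healing pickup drop is disconnected.
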(event OnSeePawn(PawnSensing)
  (params (Pawn :type Pawn%20Object%20Reference))
  (CallFunction|ChaseTarget Pawn))

(event OnDeath(Health)
  (params (HealthComponent :type Health%20Component%20Object%20Reference))
  (bind _charactermovement (Variables|Character|GetCharacterMovement))
  (if (not (Variables|Default|GetIsDead))
    (Variables|Default|SetIsDead true)
    (Variables|Default|SetcanAttack false)
    (Collision|SetActorEnableCollision false)
    (Components|Movement|StopMovementImmediately _charactermovement)
    (Pawn|Components|CharacterMovement|DisableMovement _charactermovement)
    (Development|PrintString "DEATH")
    (Animation|Montage|PlayMontage (Variables|Character|GetMesh) "/Game/LabirynthProtocol/NPC/AM_ZombieDeath.AM_ZombieDeath"
      (:OnBlendOut
        (Utilities|FlowControl|Sequence
          (:then_1
            (Actor|DestroyActor)))))))

(event Custom|Patrol
  (if (not (Variables|Default|GetIsDead))
    (AI|AIMoveTo self (.RandomLocation (AI|Navigation|GetRandomReachablePointinRadius (Transformation|GetActorLocation) 2e+03 0 0)) 0 5.0 false
      (:OnSuccess
        (Utilities|FlowControl|Delay 0.8))
      (:OnFail
        _))
    (CallFunction|Patrol)))

(event Custom|Chase%20Target
  (params (TargetActor :type Actor%20Object%20Reference))
  (bind _returnvalue (Transformation|GetActorLocation))
  (if (not (Variables|Default|GetIsDead))
    (AI|AIMoveTo self "0, 0, 0" TargetActor 5.0 false
      (:OnSuccess
        (if (Variables|Default|GetcanAttack)
          (Animation|Montage|PlayMontage (Variables|Character|GetMesh) "/Game/LabirynthProtocol/NPC/Neck_Bite_Montage.Neck_Bite_Montage"
            (:then
              (Variables|Default|SetcanAttack false))
            (:OnCompleted
              (Variables|Default|SetcanAttack true :!label _label))
            (:OnInterrupted
              (goto _label))
            (:OnNotifyBegin
              (bind (_outhit _returnvalue_2) (Collision|SphereTraceForObjects _returnvalue (+ _returnvalue (* (Math|Vector|GetForwardVector (Transformation|GetActorRotation)) 2e+02)) 2e+01 (Utilities|Array|MakeArray "ObjectTypeQuery8") false 0 "None"))
              (if _returnvalue_2
                (Utilities|IsValid (Actor|GetComponentbyClass (.HitActor (Collision|BreakHitResult _outhit)) "/Script/LabyrinthProtocol.HealthComponent")
                  (:Is%20Valid
                    (Class|HealthComponent|ApplyDamage (Actor|GetComponentbyClass (.HitActor (Collision|BreakHitResult _outhit)) "/Script/LabyrinthProtocol.HealthComponent") 10)))))))))))

(event EventBeginPlay
  (CallFunction|Patrol))

(fn ConstructionScript)
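; Collectible pickup actor that spins in the world and notifies the player when collected.
; Tick slowly yaws the skeletal mesh at a constant, frame-rate-independent rate.
; The OnPickedUped override runs the parent pickup logic, then shows a collectible-found widget on the first player's screen and plays a 2D paper-collect sound.
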(event EventBeginPlay
  (|CallParentFunction) ; This node is disabled and will not be called.\nDrag off pins to build functionality.
)

(event Collision|EventActorBeginOverlap
  (params (OtherActor :type Actor%20Object%20Reference))
  (|CallParentFunction OtherActor) ; This node is disabled and will not be called.\nDrag off pins to build functionality.
)

(event EventTick
  (params (DeltaSeconds :type Float%20%28single-precision%29))
  (|CallParentFunction DeltaSeconds)
  (Transformation|AddWorldRotation (Variables|Default|GetSkeletalMesh) (Math|Rotator|MakeRotator 0.0 0.0 (* DeltaSeconds 3e+01)) false false))

(fn ConstructionScript
  (|CallParentFunction))

(fn OnPickedUped
  (params (Player :type BP%20First%20Person%20Character%20Object%20Reference))
  (|CallParentFunction Player)
  (bind _returnvalue (UserInterface|CreateWidget "/Game/LabirynthProtocol/BP/WBP_CollectibleFOund.WBP_CollectibleFOund_C" (Game|GetPlayerController 0)))
  (UserInterface|Viewport|AddtoViewport _returnvalue 0)
  (Audio|PlaySound2D "/Game/LabirynthProtocol/Sound/paperCollect_Cue.paperCollect_Cue" 1.0 1.0 0.0 0 0))
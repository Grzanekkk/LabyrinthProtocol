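; Healing pickup that restores the player's health when collected in Labirynth Protocol.
; It overrides the parent's OnPickedUped hook to add a fixed amount to the player's Health component and play a 2D medkit sound.
; Tick spins the static mesh around its yaw axis at a steady, frame-rate-independent speed.
; Overlap detection is not implemented in this graph, whose own overlap event is a disabled stub.
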(event EventBeginPlay
  (|CallParentFunction) ; This node is disabled and will not be called.\nDrag off pins to build functionality.
)

(event Collision|EventActorBeginOverlap
  (params (OtherActor :type Actor%20Object%20Reference))
  (|CallParentFunction OtherActor) ; This node is disabled and will not be called.\nDrag off pins to build functionality.
)

(event EventTick
  (params (DeltaSeconds :type Float%20%28single-precision%29))
  (|CallParentFunction DeltaSeconds)
  (Transformation|AddWorldRotation (Variables|Default|GetStaticMesh) (Math|Rotator|MakeRotator 0.0 0.0 (* DeltaSeconds 3e+01)) false false))

(fn ConstructionScript
  (|CallParentFunction))

(fn OnPickedUped
  (params (Player :type BP%20First%20Person%20Character%20Object%20Reference))
  (|CallParentFunction Player)
  (Class|HealthComponent|AddHealth (Variables|/Game/FirstPerson/Blueprints/BP_FirstPersonCharacter.BP_FirstPersonCharacter_C|GetHealth Player) 50)
  (Audio|PlaySound2D "/Game/LabirynthProtocol/Sound/Team_Fortress_2_Medkit_sound_effect_Cue.Team_Fortress_2_Medkit_sound_effect_Cue" 1.0 1.0 0.0 0 0))
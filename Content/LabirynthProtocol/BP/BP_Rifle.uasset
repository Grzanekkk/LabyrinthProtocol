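; BP_Rifle is a rifle weapon component that supplies the visual and audio feedback for firing and reloading.
; Its fire event spawns an attached lightning muzzle effect at the muzzle socket.
; Its reload event plays a sound and attaches an electric field effect at the reload point, which a fixed timer later destroys.
; An unfinished reload movement animation is left as an empty event and unconnected nodes.
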(event Custom|ReloadAnimDown)

(event Custom|ProcessReloadFinished
  (Components|DestroyComponent (Variables|Default|GetReload%20Particle)))

(event EventBeginPlay)

(event EventTick
  (params (DeltaSeconds :type Float%20%28single-precision%29)))

(event EventProcessFiredBP
  (Niagara|SpawnSystemAttached "/Game/MixedVFX/Particles/Projectiles/NS_LightningBolt_Muzzle.NS_LightningBolt_Muzzle" self (Variables|Default|GetMuzzleSocketName) "0, 0, 0" "0, 0, 0" "KeepRelativeOffset" false))

(event EventProcessReloadedBP
  (Audio|PlaySound2D "/Game/LabirynthProtocol/Sound/QS_RifleReload.QS_RifleReload" 1.0 1.0 0.0 0 0)
  (bind _returnvalue (Niagara|SpawnSystemAttached "/Game/MixedVFX/Particles/Mix/NS_ElectricField.NS_ElectricField" self "ReloadPoint" "0, 0, 0" "0, 0, 0" "KeepRelativeOffset" false))
  (Variables|Default|SetReload%20Particle _returnvalue)
  (Utilities|Time|SetTimerbyEvent (delegate Custom|ProcessReloadFinished) 2.0))